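; BP_Conveyor is a conveyor belt that pushes the third-person player character along the direction of its Arrow component.
; Overlapping the Box stores the character and starts a looping 0.01-second timer on UpdateConveyor.
; Each call moves the character with a swept world offset of ConveyorSpeed times frame delta time, not the timer interval.
; Leaving the Box clears the reference, idling the timer without stopping it.
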(event OnComponentBeginOverlap(Box)
  (params (OverlappedComponent :type Primitive%20Component%20Object%20Reference) (OtherActor :type Actor%20Object%20Reference) (OtherComp :type Primitive%20Component%20Object%20Reference) (OtherBodyIndex :type Integer) (bFromSweep :type Boolean) (SweepResult :type Hit%20Result%20Structure%20%28by%20ref%29))
  (bind _asbp_third_person_character (Utilities|Casting|CastToBP_ThirdPersonCharacter OtherActor))
  (Variables|Default|SetPlayer _asbp_third_person_character)
  (Utilities|Time|SetTimerbyFunctionName 0 "UpdateConveyor" 0.01 true))

(event OnComponentEndOverlap(Box)
  (params (OverlappedComponent :type Primitive%20Component%20Object%20Reference) (OtherActor :type Actor%20Object%20Reference) (OtherComp :type Primitive%20Component%20Object%20Reference) (OtherBodyIndex :type Integer))
  (Utilities|Casting|CastToBP_ThirdPersonCharacter OtherActor)
  (Variables|Default|SetPlayer 0))

(fn ConstructionScript)

(fn UpdateConveyor
  (if (Utilities|IsValid (Variables|Default|GetPlayer))
    (Transformation|AddActorWorldOffset (Variables|Default|GetPlayer) (* (* (Variables|Default|GetConveyorSpeed) (Utilities|Time|GetWorldDeltaSeconds)) (Math|Vector|GetForwardVector (Variables|Default|GetArrow))) true)))